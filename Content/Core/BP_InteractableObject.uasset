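; Base Blueprint for interactable world objects that show a name prompt when the player character is nearby.
; A sphere overlap stores the ThirdPersonCharacter and shows the WBP_Interaction widget, which displays ObjectName; leaving clears both.
; While a character is in range, Tick rotates the widget toward that player's camera.
; OnInteract forwards to InteractAction, an empty function meant for child classes to override.
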(event OnComponentBeginOverlap(Sphere)
  (params (OverlappedComponent :type Primitive%20Component%20Object%20Reference) (OtherActor :type Actor%20Object%20Reference) (OtherComp :type Primitive%20Component%20Object%20Reference) (OtherBodyIndex :type Integer) (bFromSweep :type Boolean) (SweepResult :type Hit%20Result%20Structure%20%28by%20ref%29))
  ;[0 0 0] Interaction Triggers
  (bind _asthird_person_character (Utilities|Casting|CastToThirdPersonCharacter OtherActor))
  (Variables|Default|SetCharacter _asthird_person_character)
  (Rendering|SetVisibility (Variables|Default|GetWidget) true false))

(event OnComponentEndOverlap(Sphere)
  (params (OverlappedComponent :type Primitive%20Component%20Object%20Reference) (OtherActor :type Actor%20Object%20Reference) (OtherComp :type Primitive%20Component%20Object%20Reference) (OtherBodyIndex :type Integer))
  ;[0 0 0] Interaction Triggers
  (Utilities|Casting|CastToThirdPersonCharacter OtherActor)
  (Variables|Default|SetCharacter 0) ; Clear Character
  (Rendering|SetVisibility (Variables|Default|GetWidget) false false))

(event Custom|OnInteract
  (params (Character :type Character%20Object%20Reference))
  ;[0 0 0] Interaction Action - Please Override InteractionAction()
  (CallFunction|InteractAction Character))

(event EventBeginPlay
  ;[0 0 0] Begin Play
  (bind _aswbp_interaction (Utilities|Casting|CastToWBP_Interaction (UserInterface|GetUserWidgetObject (Variables|Default|GetWidget))))
  (Default|SetObjectText _aswbp_interaction (Variables|Default|GetObjectName)))

(event EventTick
  (params (DeltaSeconds :type Float%20%28single-precision%29))
  (CallFunction|UpdateWidgetRotation))

(fn ConstructionScript)

(fn InteractAction
  (params (Character :type Character%20Object%20Reference)))

(fn UpdateWidgetRotation
  (bind _character (Variables|Default|GetCharacter)
    (:then
      (bind _asplayer_controller (Utilities|Casting|CastToPlayerController (Pawn|GetController _character)))
      (Transformation|SetWorldRotation (Variables|Default|GetWidget) (Math|Rotator|FindLookatRotation (Transformation|GetWorldLocation (Variables|Default|GetWidget)) (Camera|GetCameraLocation (Variables|/Script/Engine.PlayerController|GetPlayerCameraManager _asplayer_controller))) false false))
    (:else)))