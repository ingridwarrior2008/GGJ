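; BP_MovableLight is a spotlight that slides back and forth along a spline in response to move up, move down and release events.
; The move events set a direction and enable movement on Tick, and release stops it.
; When UseSpline is set, MoveOnSpline places the light at the stored distance, then advances that distance by Speed times delta time, clamped to the spline's ends.
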(event Custom|OnMoveUp
  (params (Character :type Character%20Object%20Reference))
  (Variables|Default|SetIsMoving true)
  (Variables|Default|SetCanMoveUp true))

(event Custom|OnMoveDown
  (params (Character :type Character%20Object%20Reference))
  (Variables|Default|SetIsMoving true)
  (Variables|Default|SetCanMoveUp false))

(event Custom|OnRelease
  (Variables|Default|SetIsMoving false))

(event EventBeginPlay)

(event EventTick
  (params (DeltaSeconds :type Float%20%28single-precision%29))
  (if (Variables|Default|GetIsMoving)
    (Utilities|FlowControl|Sequence
      (:then_0
        (|MoveOnSpline DeltaSeconds)))))

(fn ConstructionScript)