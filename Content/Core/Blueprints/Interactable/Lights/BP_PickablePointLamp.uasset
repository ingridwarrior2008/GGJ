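; Pickable point lamp interactable that a character can grab and release.
; On interact, it attaches to the character's lamp socket with a grabbing montage and blanks the interaction UI's object and key text.
; On release, it detaches with the physics and collision enable flags off, then restores the prompt from its object and key names.
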(event EventBeginPlay
  (|CallParentFunction) ; This node is disabled and will not be called.\nDrag off pins to build functionality.
)

(event Collision|EventActorBeginOverlap
  (params (OtherActor :type Actor%20Object%20Reference)))

(event EventTick
  (params (DeltaSeconds :type Float%20%28single-precision%29))
  (|CallParentFunction DeltaSeconds) ; This node is disabled and will not be called.\nDrag off pins to build functionality.
)

(event EventOnInteract
  (params (Character :type Character%20Object%20Reference))
  (bind _interactionui (Variables|Default|GetInteractionUI))
  (CallFunction|AttachInteractable Character "LampSocket" "/Game/Mannequin/Animations/AM_GrabbingLamp.AM_GrabbingLamp")
  (Default|SetObjectText _interactionui)
  (Default|SetKeyText _interactionui))

(event EventOnReleasedInteract
  (params (Character :type Character%20Object%20Reference))
  (bind _interactionui (Variables|Default|GetInteractionUI))
  (CallFunction|DetachInteractable Character false false)
  (Default|SetObjectText _interactionui (Variables|Default|GetObjectName))
  (Default|SetKeyText _interactionui (Variables|Default|GetKeyName)))

(fn ConstructionScript
  (|CallParentFunction))