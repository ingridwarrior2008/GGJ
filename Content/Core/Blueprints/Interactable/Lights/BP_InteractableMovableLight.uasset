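; BP_InteractableMovableLight is an interactable that lets a character move a referenced movable light up or down.
; Its move-up and move-down interact events forward to MovableLights, with move-down also passing the interacting Character.
; Both release events call the same OnRelease on MovableLights.
; Every call is guarded by a validity check, and the Blueprint holds no movement logic of its own.
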(event EventBeginPlay
  (|CallParentFunction) ; This node is disabled and will not be called.\nDrag off pins to build functionality.
)

(event Collision|EventActorBeginOverlap
  (params (OtherActor :type Actor%20Object%20Reference)))

(event EventTick
  (params (DeltaSeconds :type Float%20%28single-precision%29))
  (|CallParentFunction DeltaSeconds) ; This node is disabled and will not be called.\nDrag off pins to build functionality.
)

(event EventOnReleasedMoveUp
  (params (Character :type Character%20Object%20Reference))
  (bind _movablelights (Variables|Default|GetMovableLights)
    (:then
      (Default|OnRelease _movablelights))
    (:else)))

(event EventOnReleaseMoveDown
  (params (Character :type Character%20Object%20Reference))
  (bind _movablelights (Variables|Default|GetMovableLights)
    (:then
      (Default|OnRelease _movablelights))
    (:else)))

(event EventOnInteractMoveUp
  (params (Character :type Character%20Object%20Reference))
  (bind _movablelights (Variables|Default|GetMovableLights)
    (:then
      (Default|OnMoveUp _movablelights))
    (:else)))

(event EventOnInteractMoveDown
  (params (Character :type Character%20Object%20Reference))
  (bind _movablelights (Variables|Default|GetMovableLights)
    (:then
      (Default|OnMoveDown _movablelights Character))
    (:else)))

(fn ConstructionScript
  (|CallParentFunction))